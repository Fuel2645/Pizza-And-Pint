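; Actor component for a player ranking system that maps the player's RankingScore to Unranked, C, B, A or S.
; BeginPlay caches the Charater1 player and seeds a starting score.
; Each Tick checks score bands, with small gaps at their boundaries, and RankChange prints the matching DT_RankSystem row's rank.
; Tick then cuts the score by a fixed percentage, so decay is exponential and frame-rate dependent.
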(event `self.ReceiveBeginPlay`
  (bind _ascharater_1 (cast `/Game/Daniel/Charater1` (`GameplayStatics.GetPlayerCharacter` 0)))
  (bind _output_get (set `self.PlayerRef` _ascharater_1))
  (set `/Game/Daniel/Charater1.RankingScore` 3000 _output_get))

(event `RankChange`
  (params (CurrentRankID :type Integer))
  (bind _returnvalue (`|GetDataTableRow` "/Game/Ashley/RankSystem/DT_RankSystem.DT_RankSystem" (select `int` CurrentRankID :`0` "Unranked" :`1` "C" :`2` "B" :`3` "A" :`4` "S" :!type "Name"))
    (:`then`
      (bind _output_get (set `self.F_RankSystem` _returnvalue))
      (`KismetSystemLibrary.PrintString` (`KismetStringLibrary.Conv_NameToString` (`.Rank_7_C006EFD44BF35747CACD1EB377DCC561` (break `/Game/Ashley/RankSystem/F_RankSystem` _output_get)))))))

(event `self.ReceiveTick`
  (params (DeltaSeconds :type "Float (single-precision)"))
  (bind _playerref (`self.PlayerRef`))
  (bind _rankingscore (`/Game/Daniel/Charater1.RankingScore` (`self.PlayerRef`)))
  (bind _rankingscore_2 (`/Game/Daniel/Charater1.RankingScore` (`self.PlayerRef`)))
  (bind _rankingscore_3 (`/Game/Daniel/Charater1.RankingScore` (`self.PlayerRef`)))
  (bind _rankingscore_4 (`/Game/Daniel/Charater1.RankingScore` (`self.PlayerRef`)))
  (`|ExecutionSequence`
    (:`then_0`
      (if (<= (`/Game/Daniel/Charater1.RankingScore` (`self.PlayerRef`)) 300)
        (`self.RankChange` 0)
        (elif (and (<= _rankingscore 700) (> _rankingscore 301))
          (`self.RankChange` 1)
          (elif (and (> _rankingscore_3 701) (<= _rankingscore_3 1200))
            (`self.RankChange` 2)
            (elif (and (> _rankingscore_2 1201) (<= _rankingscore_2 1900))
              (`self.RankChange` 3)
              (elif (and (> _rankingscore_4 1901) (<= _rankingscore_4 9999))
                (`self.RankChange` 4)))))))
    (:`then_1`
      (set `/Game/Daniel/Charater1.RankingScore` (- (`/Game/Daniel/Charater1.RankingScore` _playerref) (* (`/Game/Daniel/Charater1.RankingScore` (`self.PlayerRef`)) 0.05)) _playerref))))