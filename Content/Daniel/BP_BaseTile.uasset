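; BP_BaseTile is a base tile Blueprint that records the world positions of its four door points.
; The Construction Script reads the world location of the First, Second, Third and Fourth components and appends each to the DoorLocations array.
; The array is not cleared in the script before appending, and the event graph holds no active logic.
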(fn `UserConstructionScript`
  (bind _door_locations (`self.Door Locations`))
  (`BlueprintMapLibrary.Map_Add` _door_locations (`SceneComponent.K2_GetComponentLocation` (`self.First`)))
  (`BlueprintMapLibrary.Map_Add` _door_locations (`SceneComponent.K2_GetComponentLocation` (`self.Second`)))
  (`BlueprintMapLibrary.Map_Add` _door_locations (`SceneComponent.K2_GetComponentLocation` (`self.Third`)))
  (`BlueprintMapLibrary.Map_Add` _door_locations (`SceneComponent.K2_GetComponentLocation` (`self.Fourth`))))