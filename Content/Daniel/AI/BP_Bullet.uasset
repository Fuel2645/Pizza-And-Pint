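; BP_Bullet is a projectile that damages AI and character actors on contact.
; InitaliseStuff takes bullet stats, storing the damage and setting the projectile movement's initial and max speed.
; When its Box begins overlapping an actor whose class is exactly BP_AI or Charater, it applies that damage and destroys itself.
; Overlaps with any other class, child classes included, are ignored.
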(event `self.Box.OnComponentBeginOverlap`
  (params (OverlappedComponent :type "PrimitiveComponent Object Reference") (OtherActor :type "Actor Object Reference") (OtherComp :type "PrimitiveComponent Object Reference") (OtherBodyIndex :type Integer) (bFromSweep :type Boolean) (SweepResult :type "HitResult Structure (by ref)"))
  (bind _returnvalue (`GameplayStatics.GetObjectClass` OtherActor))
  (if (or (== _returnvalue "/Game/Daniel/AI/BP_AI.BP_AI_C") (== _returnvalue "/Game/JJ/Charater.Charater_C"))
    (`GameplayStatics.ApplyDamage` OtherActor (`self.Damage`))
    (`self.K2_DestroyActor`)))

(event `Initalise Stuff`
  (params (BulletStats :type "/Game/Daniel/AI/ST_Bullets Structure"))
  (bind _projectilemovement (`self.ProjectileMovement`))
  (set `self.Damage` BulletStats_Damage_2_A32D19AA4A8366EF68C260BEE83F186E)
  (set `ProjectileMovementComponent.InitialSpeed` BulletStats_Speed_4_335A258449E2C8745F95E4AB152AF329 _projectilemovement)
  (set `ProjectileMovementComponent.MaxSpeed` BulletStats_Speed_4_335A258449E2C8745F95E4AB152AF329 _projectilemovement))

(fn `UserConstructionScript`)