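; Enemy AI that chases the player, fires bullet bursts, and on death drops BP_Bottle and awards score scaled by the "Unranked" rank multiplier.
; A looping timer moves it toward the player until AIPerception senses them inside its Sphere, triggering Attack.
; Attack turns toward the player over repeated timer ticks, picks a random DT_Bullet_Types row for burst count and delay, spawns BP_Bullets, then shifts to a nearby random point before resetting.
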(event `self.ReceiveBeginPlay`
  (bind (_returnvalue_roll _returnvalue_pitch) (`KismetMathLibrary.BreakRotator` (`SceneComponent.K2_GetComponentRotation` (`self.CapsuleComponent`))))
  (bind (_returnvalue_roll_2 _returnvalue_pitch_2 _returnvalue_yaw) (`KismetMathLibrary.BreakRotator` (`KismetMathLibrary.FindLookAtRotation` (`SceneComponent.K2_GetComponentLocation` (`self.Mesh`)) (`self.K2_GetActorLocation` (`GameplayStatics.GetPlayerCharacter` 0)))))
  (bind _ascharater_1 (cast `/Game/Daniel/Charater1` (`GameplayStatics.GetPlayerCharacter` 0)))
  (set `self.As Charater 1` _ascharater_1)
  (bind _returnvalue (`|GetDataTableRow` "/Game/Ashley/RankSystem/DT_RankSystem.DT_RankSystem" "Unranked")
    (:`then`
      (set `self.F_RankSystem` _returnvalue)
      (`SceneComponent.K2_SetWorldRotation` (`self.CapsuleComponent`) (`KismetMathLibrary.MakeRotator` _returnvalue_roll _returnvalue_pitch _returnvalue_yaw) false false)
      (`KismetSystemLibrary.K2_SetTimerDelegate` (delegate `AI_Loop`) 0.1 true))))

(event `AI_Loop`
  (if (and (`self.FoundPlayer`) (`self.PlayerInRange`))
    (if (not (`self.IsFiring`))
      (set `self.IsFiring` true)
      (`self.Attack`))
    (else
      (`|AIMoveTo` self (0.0 0.0 0.0) (`GameplayStatics.GetPlayerCharacter` 0) (/ (`SphereComponent.SphereRadius` (`self.Sphere`)) 2.0)))))

(event `self.Sphere.OnComponentBeginOverlap`
  (params (OverlappedComponent :type "PrimitiveComponent Object Reference") (OtherActor :type "Actor Object Reference") (OtherComp :type "PrimitiveComponent Object Reference") (OtherBodyIndex :type Integer) (bFromSweep :type Boolean) (SweepResult :type "HitResult Structure (by ref)"))
  (if (== OtherActor (`GameplayStatics.GetPlayerCharacter` 0))
    (set `self.PlayerInRange` true)))

(event `self.Sphere.OnComponentEndOverlap`
  (params (OverlappedComponent :type "PrimitiveComponent Object Reference") (OtherActor :type "Actor Object Reference") (OtherComp :type "PrimitiveComponent Object Reference") (OtherBodyIndex :type Integer))
  (if (== OtherActor (`GameplayStatics.GetPlayerCharacter` 0))
    (set `self.PlayerInRange` false)))

(event `Attack`
  (bind (_bullet_stats_damage _bullet_stats_speed _bullet_stats_numberofbulletsfired _bullet_stats_delaybetweenshooting) (break `/Game/Daniel/AI/ST_Bullets` (`self.Bullet Stats`)))
  (bind _arrow1 (`self.Arrow1`))
  (bind (_returnvalue_roll _returnvalue_pitch) (`KismetMathLibrary.BreakRotator` (`SceneComponent.K2_GetComponentRotation` (`self.CapsuleComponent`))))
  (bind (_returnvalue_roll_2 _returnvalue_pitch_2 _returnvalue_yaw) (`KismetMathLibrary.BreakRotator` (`KismetMathLibrary.FindLookAtRotation` (`SceneComponent.K2_GetComponentLocation` (`self.Mesh`)) (`self.K2_GetActorLocation` (`GameplayStatics.GetPlayerCharacter` 0)))))
  (`/Engine/EditorBlueprintResources/StandardMacros.IsValid` self
    (:`Is Valid`
      (`|AIMoveTo` self (`SceneComponent.K2_GetComponentLocation` (`self.CapsuleComponent`)) null
        (:`then`
          (bind _returnvalue (`KismetSystemLibrary.K2_SetTimerDelegate` (delegate `Attack`) 0.1 true))
          (`SceneComponent.K2_SetWorldRotation` (`self.CapsuleComponent`) (`KismetMathLibrary.MakeRotator` _returnvalue_roll _returnvalue_pitch _returnvalue_yaw) false false)
          (bind _result (`/Engine/EditorBlueprintResources/StandardMacros.IncrementInt` (`self.LoopCOunt`))
            (:`  `
              (if (not (<= _result 3))
                (`KismetSystemLibrary.K2_PauseTimerHandle` _returnvalue)
                (`self.Change Bullet`)
                (if (== (`self.BulletLoopCOunt`) _bullet_stats_numberofbulletsfired) :!label _label
                  (`KismetSystemLibrary.Delay` 0.2)
                  (`|AIMoveTo` self (`NavigationSystemV1.K2_GetRandomReachablePointInRadius` (`SceneComponent.K2_GetComponentLocation` (`self.CapsuleComponent`)) 50.0 null null) null
                    (:`OnSuccess`
                      (set `self.IsFiring` false)
                      (set `self.LoopCOunt` 0)
                      (set `self.BulletLoopCOunt` 0)
                      (set `self.isMoving` false)))
                  (else
                    (`/Engine/EditorBlueprintResources/StandardMacros.IsValid` _arrow1
                      (:`Is Valid`
                        (`|SpawnActorFromClass` "/Game/Daniel/AI/BP_Bullet.BP_Bullet_C" (`KismetMathLibrary.MakeTransform` (+ (`SceneComponent.K2_GetComponentLocation` _arrow1) (* (`SceneComponent.GetForwardVector` _arrow1) 20.0)) (`SceneComponent.K2_GetComponentRotation` _arrow1)) "Undefined" "MultiplyWithRoot" null null)
                        (`KismetSystemLibrary.Delay` _bullet_stats_delaybetweenshooting)
                        (`/Engine/EditorBlueprintResources/StandardMacros.IncrementInt` (`self.BulletLoopCOunt`)
                          (:`  `
                            (goto _label)))))))))))))))

(event `self.AIPerception.OnTargetPerceptionUpdated`
  (params (Actor :type "Actor Object Reference") (Stimulus :type "AIStimulus Structure"))
  (if (== Actor (`GameplayStatics.GetPlayerCharacter` 0))
    (if Stimulus_bSuccessfullySensed
      (set `self.FoundPlayer` true)
      (else
        (set `self.FoundPlayer` false)))))

(event `self.AIPerception.OnTargetPerceptionForgotten`
  (params (Actor :type "Actor Object Reference"))
  (if (== Actor (`GameplayStatics.GetPlayerCharacter` 0))
    (set `self.FoundPlayer` false)))

(event `Change Bullet`
  (bind _outrownames (`DataTableFunctionLibrary.GetDataTableRowNames` "/Game/Daniel/AI/DT_Bullet_Types.DT_Bullet_Types"))
  (bind _returnvalue (`|GetDataTableRow` "/Game/Daniel/AI/DT_Bullet_Types.DT_Bullet_Types" (`KismetArrayLibrary.Array_Random` _outrownames))
    (:`then`
      (set `self.Bullet Stats` _returnvalue))))

(event `self.ReceiveAnyDamage`
  (params (Damage :type "Float (single-precision)") (DamageType :type "DamageType Object Reference") (InstigatedBy :type "Controller Object Reference") (DamageCauser :type "Actor Object Reference"))
  (bind (_f_ranksystem_rank _f_ranksystem_scoremult) (break `/Game/Ashley/RankSystem/F_RankSystem` (`self.F_RankSystem`)))
  (bind _as_charater_1 (`self.As Charater 1`))
  (bind _output_get (set `self.Health` (- (`self.Health`) Damage)))
  (if (<= _output_get 0.0)
    (`|SpawnActorFromClass` "/Game/Daniel/BP_Bottle.BP_Bottle_C" (`KismetMathLibrary.MakeTransform` (`SceneComponent.K2_GetComponentLocation` (`self.CapsuleComponent`))) "Undefined" "MultiplyWithRoot" null null)
    (`self.K2_DestroyActor`)
    (set `/Game/Daniel/Charater1.Score` (+ (`/Game/Daniel/Charater1.Score` _as_charater_1) (* 100 _f_ranksystem_scoremult)) _as_charater_1)
    (`self.K2_DestroyActor`)))

(fn `UserConstructionScript`)