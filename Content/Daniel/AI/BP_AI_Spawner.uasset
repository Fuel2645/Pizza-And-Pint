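; BP_AI_Spawner is a spawner actor that repeatedly creates BP_AI actors while the game runs.
; On BeginPlay it starts a looping timer at the SpawnRate interval, which fires the SpawnAI event.
; Each firing loops up to SpawnCount, spawning at the Arrow component's world location with a small random horizontal offset.
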(event `self.ReceiveBeginPlay`
  (`KismetSystemLibrary.K2_SetTimerDelegate` (delegate `Spawn AI`) (`self.SpawnRate`) true))

(event `Spawn AI`
  (for _ (range (+ (`self.SpawnCount`) 1))
    (`|SpawnActorFromClass` "/Game/Daniel/AI/BP_AI.BP_AI_C" (`KismetMathLibrary.MakeTransform` (+ (`SceneComponent.K2_GetComponentLocation` (`self.Arrow`)) (`KismetMathLibrary.MakeVector` (`KismetMathLibrary.RandomFloatInRange` -20.0 20.0) (`KismetMathLibrary.RandomFloatInRange` -20.0 20.0)))) "Undefined" "MultiplyWithRoot" null null)))

(fn `UserConstructionScript`)