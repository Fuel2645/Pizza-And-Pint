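; BP_TileManager is an unfinished procedural room layout generator that spawns map tiles on BeginPlay.
; It places a first tile, then walks each tile's DoorLocations map and spawns neighbors 950 units out from unconnected doors, choosing direction by door index.
; A separate SpawnPanel function does the same offset spawn with BP_BaseTile_Child and records it in MapTiles, but BeginPlay never calls it or records its neighbor spawns.
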(event `self.ReceiveBeginPlay`
  (if (== (`KismetArrayLibrary.Array_Length` (`self.MapTiles`)) (`KismetMathLibrary.RandomIntegerInRange` (`self.Min Num Rooms`) (`self.Max Num Rooms`))) :!label _label
    _
    (elif (`self.FirstRoom`)
      (bind _returnvalue (`|SpawnActorFromClass` :`Class` "/Game/Daniel/BP_BaseTile.BP_BaseTile_C" :`SpawnTransform` (`KismetMathLibrary.MakeTransform` (0.0 0.0 0.0)) :`CollisionHandlingOverride` "AlwaysSpawn" :`TransformScaleMethod` "MultiplyWithRoot" :`Instigator` null))
      (set `self.FirstRoom` false)
      (`KismetArrayLibrary.Array_Add` (`self.MapTiles`) _returnvalue)
      (goto _label)
      (else
        (for _array_element (`self.MapTiles`)
          (bind _door_locations (`/Game/Daniel/BP_BaseTile.Door Locations` _array_element))
          (bind _values (`BlueprintMapLibrary.Map_Values` _door_locations))
          (for (_array_element_2 _array_index) _values
            (if _array_element_2
              (`KismetSystemLibrary.PrintString` "Door Already Connected/Blocked")
              (else
                (bind _keys (`BlueprintMapLibrary.Map_Keys` _door_locations))
                (switch `int` _array_index
                  (:`Default`
                    (`KismetSystemLibrary.PrintString` "Error"))
                  (:`0`
                    (bind _output (`|GetArrayItem` _keys _array_index))
                    (bind _output_get (set `self.TileMovement` (+ _output (-950.0 0.0 0.0))))
                    (`BlueprintMapLibrary.Map_Add` _door_locations _output_get true)
                    (`|SpawnActorFromClass` :`Class` "/Game/Daniel/BP_BaseTile_Child.BP_BaseTile_Child_C" :`SpawnTransform` (`KismetMathLibrary.MakeTransform` (`self.TileMovement`)) :`CollisionHandlingOverride` "Undefined" :`TransformScaleMethod` "MultiplyWithRoot" :`Instigator` null :!label _label_2))
                  (:`1`
                    (bind _output_get_2 (set `self.TileMovement` (+ _output (950.0 0.0 0.0))))
                    (`BlueprintMapLibrary.Map_Add` _door_locations _output_get_2 true)
                    (goto _label_2))
                  (:`2`
                    (bind _output_get_3 (set `self.TileMovement` (+ _output (0.0 950.0 0.0))))
                    (`BlueprintMapLibrary.Map_Add` _door_locations _output_get_3 true)
                    (goto _label_2))
                  (:`3`
                    (bind _output_get_4 (set `self.TileMovement` (+ _output (0.0 -950.0 0.0))))
                    (`BlueprintMapLibrary.Map_Add` _door_locations _output_get_4 true)
                    (goto _label_2)))))))))))

(fn `Spawn Panel`
  (params (Selection :type Integer) (TargetMap :type "Map of Vector Structure to Boolean (by ref)"))
  (bind _keys (`BlueprintMapLibrary.Map_Keys` TargetMap))
  (switch `int` Selection
    (:`0`
      (bind _output (`|GetArrayItem` _keys Selection))
      (set `self.TileMovement` (+ _output (-950.0 0.0 0.0))))
    (:`1`
      (set `self.TileMovement` (+ _output (950.0 0.0 0.0))))
    (:`2`
      (set `self.TileMovement` (+ _output (0.0 950.0 0.0))))
    (:`3`
      (set `self.TileMovement` (+ _output (0.0 -950.0 0.0)))))
  (`BlueprintMapLibrary.Map_Add` TargetMap _output true)
  (bind _returnvalue (`|SpawnActorFromClass` :`Class` "/Game/Daniel/BP_BaseTile_Child.BP_BaseTile_Child_C" :`SpawnTransform` (`KismetMathLibrary.MakeTransform` (`self.TileMovement`)) :`CollisionHandlingOverride` "Undefined" :`TransformScaleMethod` "MultiplyWithRoot" :`Instigator` null))
  (`KismetArrayLibrary.Array_Add` (`self.MapTiles`) _returnvalue))

(fn `UserConstructionScript`)