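; BP_BaseTile is a base tile actor with four door slots that are shown or hidden according to their states.
; The construction script fills the DoorStates map, keyed by each door component's world location, with state 0.
; DoorCheck prints each value and, matching components by map order, hides those at state 1 and shows the rest.
; BeginPlay spawns a PlayerStart at the tile's stored start point.
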(event `self.ReceiveBeginPlay`
  (`|SpawnActorFromClass` "/Script/Engine.PlayerStart" (`KismetMathLibrary.MakeTransform` (`self.Player Start`)) "Undefined" "MultiplyWithRoot" null null))

(event `DoorCheck`
  (bind _values (`BlueprintMapLibrary.Map_Values` (`self.Door States`)))
  (for (_array_element _array_index) _values
    (`KismetSystemLibrary.PrintString` (`KismetStringLibrary.Conv_IntToString` _array_element))
    (if (!= _array_element 1)
      (switch `int` _array_index
        (:`0`
          (`SceneComponent.SetHiddenInGame` (`self.First`) false true))
        (:`1`
          (`SceneComponent.SetHiddenInGame` (`self.Second`) false true))
        (:`2`
          (`SceneComponent.SetHiddenInGame` (`self.Third`) false true))
        (:`3`
          (`SceneComponent.SetHiddenInGame` (`self.Fourth`) false true)))
      (else
        (switch `int` _array_index
          (:`0`
            (`SceneComponent.SetHiddenInGame` (`self.First`) true true))
          (:`1`
            (`SceneComponent.SetHiddenInGame` (`self.Second`) true true))
          (:`2`
            (`SceneComponent.SetHiddenInGame` (`self.Third`) true true))
          (:`3`
            (`SceneComponent.SetHiddenInGame` (`self.Fourth`) true true)))))))

(fn `UserConstructionScript`
  (bind _door_states (`self.Door States`))
  (`BlueprintMapLibrary.Map_Add` _door_states (`SceneComponent.K2_GetComponentLocation` (`self.First`)))
  (`BlueprintMapLibrary.Map_Add` _door_states (`SceneComponent.K2_GetComponentLocation` (`self.Second`)))
  (`BlueprintMapLibrary.Map_Add` _door_states (`SceneComponent.K2_GetComponentLocation` (`self.Third`)))
  (`BlueprintMapLibrary.Map_Add` _door_states (`SceneComponent.K2_GetComponentLocation` (`self.Fourth`))))