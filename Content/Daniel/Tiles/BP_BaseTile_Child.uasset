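; BP_BaseTile_Child is a tile variant that sets the states of its doors in the inherited construction flow and on creation.
; The construction script runs the parent's, then gives each DoorStates key a 50% chance of state 2.
; The Created event takes an Index and sets the paired door (0↔1, 2↔3) to state 1.
; Logic that hides the First to Fourth components is disconnected and never runs.
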(event `Created`
  (params (Index :type Integer))
  (bind _door_states (`self.Door States`))
  (bind _keys (`BlueprintMapLibrary.Map_Keys` _door_states))
  (switch `int` Index
    (:`0`
      (`BlueprintMapLibrary.Map_Add` _door_states (`|GetArrayItem` _keys 1) 1))
    (:`1`
      (`BlueprintMapLibrary.Map_Add` _door_states (`|GetArrayItem` _keys) 1))
    (:`2`
      (`BlueprintMapLibrary.Map_Add` _door_states (`|GetArrayItem` _keys 3) 1))
    (:`3`
      (`BlueprintMapLibrary.Map_Add` _door_states (`|GetArrayItem` _keys 2) 1))))

(fn `UserConstructionScript`
  (bind _door_states (`self.Door States`))
  (`parent.UserConstructionScript`)
  (bind _keys (`BlueprintMapLibrary.Map_Keys` _door_states))
  (for _array_element _keys
    (if (== (`KismetMathLibrary.RandomInteger` 2) 0)
      (`BlueprintMapLibrary.Map_Add` _door_states _array_element 2))))