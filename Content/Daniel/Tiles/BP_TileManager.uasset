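; Tile manager that procedurally builds a room map on BeginPlay, targeting a fixed tile count.
; It spawns a base tile, then walks the growing tile array, spawning random child tiles offset from open doors by direction.
; DoorValidation then propagates connected states to shared door positions before each tile runs DoorCheck.
; A temporary-box overlap test runs before each spawn, but its result handling is disconnected.
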(event `self.ReceiveBeginPlay`
  (bind _maptiles (`self.MapTiles`))
  (bind _maptiles_2 (`self.MapTiles`))
  (bind _output_get (set `self.RoomSize` 20))
  (if (== (`KismetArrayLibrary.Array_Length` (`self.MapTiles`)) _output_get) :!label _label
    _
    (elif (`self.FirstRoom`)
      (bind _returnvalue (`|SpawnActorFromClass` "/Game/Daniel/Tiles/BP_BaseTile.BP_BaseTile_C" (`KismetMathLibrary.MakeTransform` (0.0 0.0 0.0)) "AlwaysSpawn" "MultiplyWithRoot" null null))
      (set `self.FirstRoom` false)
      (`KismetArrayLibrary.Array_Add` (`self.MapTiles`) _returnvalue)
      (goto _label)
      (else
        (for _array_element _maptiles_2 :!label _label_2
          (bind _door_states (`/Game/Daniel/Tiles/BP_BaseTile.Door States` _array_element))
          (bind _values (`BlueprintMapLibrary.Map_Values` _door_states))
          (for (_array_element_2 _array_index) _values
            (if (!= _array_element_2 0)
              (`KismetSystemLibrary.PrintString` "Door Already Connected/Blocked")
              (else
                (bind _keys (`BlueprintMapLibrary.Map_Keys` _door_states))
                (switch `int` _array_index
                  (:`Default`
                    (`KismetSystemLibrary.PrintString` "Error"))
                  (:`0`
                    (bind _output (`|GetArrayItem` _keys _array_index))
                    (bind _output_get_2 (set `self.TileMovement` (+ _output (-1000.0 0.0 0.0))))
                    (bind (_box _isoverlapping) (`self.OverlapCheck` _array_element _output_get_2))
                    (bind _returnvalue_2 (`|SpawnActorFromClass` (`KismetArrayLibrary.Array_Random` (`self.RandomTile`)) (`KismetMathLibrary.MakeTransform` (`self.TileMovement`)) "Undefined" "MultiplyWithRoot" null null :!label _label_3))
                    (bind _asbp_base_tile_child (cast `/Game/Daniel/Tiles/BP_BaseTile_Child` _returnvalue_2))
                    (`/Game/Daniel/Tiles/BP_BaseTile_Child.Created` _asbp_base_tile_child _array_index)
                    (`KismetArrayLibrary.Array_Add` _maptiles _asbp_base_tile_child)
                    (if (== (`KismetArrayLibrary.Array_Length` _maptiles) (`self.RoomSize`))
                      (`|ExecutionSequence`
                        (:`then_0`
                          (break))
                        (:`then_1`
                          (goto _label_2 :!via `Break`)))))
                  (:`1`
                    (bind _output_get_3 (set `self.TileMovement` (+ _output (1000.0 0.0 0.0))))
                    (bind (_box_2 _isoverlapping_2) (`self.OverlapCheck` _array_element _output_get_3))
                    (goto _label_3))
                  (:`2`
                    (bind _output_get_4 (set `self.TileMovement` (+ _output (0.0 1000.0 0.0))))
                    (bind (_box_3 _isoverlapping_3) (`self.OverlapCheck` _array_element _output_get_4))
                    (goto _label_3))
                  (:`3`
                    (bind _output_get_5 (set `self.TileMovement` (+ _output (0.0 -1000.0 0.0))))
                    (bind (_box_4 _isoverlapping_4) (`self.OverlapCheck` _array_element _output_get_5))
                    (goto _label_3)))))))
        (for _array_element_3 _maptiles_2
          (bind _door_states_2 (`/Game/Daniel/Tiles/BP_BaseTile.Door States` _array_element_3))
          (bind _values_2 (`BlueprintMapLibrary.Map_Values` _door_states_2))
          (for (_array_element_4 _array_index_2) _values_2
            (if (== _array_element_4 1)
              (bind _keys_2 (`BlueprintMapLibrary.Map_Keys` _door_states_2))
              (for _array_element_5 _maptiles_2
                (if (not (== _array_element_3 _array_element_5))
                  (bind _door_states_3 (`/Game/Daniel/Tiles/BP_BaseTile.Door States` _array_element_5))
                  (bind _output_2 (`|GetArrayItem` _keys_2 _array_index_2))
                  (if (`.ReturnValue` (`BlueprintMapLibrary.Map_Find` _door_states_3 _output_2))
                    (`BlueprintMapLibrary.Map_Add` _door_states_3 _output_2 1)))))))
        (for _array_element_6 _maptiles_2
          (`/Game/Daniel/Tiles/BP_BaseTile.DoorCheck` _array_element_6))))))

(fn `OverlapCheck`
  (params (BaseTile :type "Actor Object Reference") (Location :type "Vector Structure"))
  (returns (Box :type "BoxComponent Object Reference") (ISOverlapping :type Boolean))
  (bind _returnvalue (`AddComponent|NODE_AddBoxComponent-1` :`RelativeTransform` (`KismetMathLibrary.MakeTransform` Location)))
  (for _array_element (`self.GetAllChildActors` BaseTile true)
    (bind _returnvalue_2 (`PrimitiveComponent.IsOverlappingActor` _returnvalue _array_element))
    (if _returnvalue_2
      (break)))
  (return _returnvalue _returnvalue_2))

(fn `UserConstructionScript`)